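; Player character for a 2D side-scroller, with run, jump, dash, melee attack, health potions and sword pickup.
; Stamina regenerates on Tick and gates jump, dash and attack, while setters clamp stats and update the WB_Main HUD.
; Tick also picks flipbooks from state and triggers hitbox damage once on attack frame 2, reset when playback finishes.
; Death shows WB_Death and turns the jump input into a level restart.
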(event OnFinishedPlaying(Sprite)
  (if (== (Variables|Default|GetisAttacking) true)
    (Variables|Default|SetisAttacking false)
    (CallFunction|ResetAttack)))

(event Custom|Death
  (Variables|Default|SetisDead true)
  (bind _returnvalue (UserInterface|CreateWidget "/Game/UI/WB_Death.WB_Death_C"))
  (UserInterface|Viewport|AddtoViewport _returnvalue 0))

(event Custom|Reset%20Attack
  ;[1 1 1] Атака
  (Utilities|FlowControl|DoOnce false) ; enters at Reset
)

(event Input|EnhancedActionEvents|EnhancedInputActionIA_Move
  (params (ActionValue :type Float%20%28double-precision%29) (ElapsedSeconds :type Float%20%28double-precision%29) (TriggeredSeconds :type Float%20%28double-precision%29) (InputAction :type Input%20Action%20Object%20Reference :default "/Game/Input/Actions/IA_Move.IA_Move"))
  (if (Math|Boolean|NORBoolean (Variables|Default|GetisAttacking) (Variables|Default|GetisDead))
    (Pawn|Input|AddMovementInput "0.500000,0.000000,0.000000" ActionValue false)
    (Pawn|SetControlRotation (Pawn|GetController) (select (> ActionValue 0.0) (Math|Rotator|MakeRotator 0.0 0.0 0.0) (Math|Rotator|MakeRotator 0.0 0.0 1.8e+02)))))

(event Input|EnhancedActionEvents|EnhancedInputActionIA_Jump
  (params (ActionValue :type Boolean) (ElapsedSeconds :type Float%20%28double-precision%29) (TriggeredSeconds :type Float%20%28double-precision%29) (InputAction :type Input%20Action%20Object%20Reference :default "/Game/Input/Actions/IA_Jump.IA_Jump"))
  ;[1 1 1] Прыжок / рестарт
  (:Started
    (if (Variables|Default|GetisDead)
      (CallFunction|RestartLevel)
      (else
        (bind _value (CallFunction|CheckCanDoAction 2e+01))
        (if _value
          (Character|Jump))))))

(event Input|EnhancedActionEvents|EnhancedInputActionIA_Attack
  (params (ActionValue :type Boolean) (ElapsedSeconds :type Float%20%28double-precision%29) (TriggeredSeconds :type Float%20%28double-precision%29) (InputAction :type Input%20Action%20Object%20Reference :default "/Game/Input/Actions/IA_Attack.IA_Attack"))
  (:Started
    (bind _value (CallFunction|CheckCanDoAction 25.0))
    (if _value
      (if (AI|Components|NavMovement|IsMovingonGround (Variables|Character|GetCharacterMovement))
        (Variables|Default|SetisAttacking true)
        (CallFunction|SetStamina (- (Variables|Default|GetcurrentStamina) 25.0))))))

(event Input|EnhancedActionEvents|EnhancedInputActionIA_UseHealthPotion
  (params (ActionValue :type Boolean) (ElapsedSeconds :type Float%20%28double-precision%29) (TriggeredSeconds :type Float%20%28double-precision%29) (InputAction :type Input%20Action%20Object%20Reference :default "/Game/Input/Actions/IA_UseHealthPotion.IA_UseHealthPotion"))
  ;[1 1 1] Взаимодействие с зельями здоровья
  (:Started
    (bind _result (Math|Integer|DecrementInt (Variables|Default|GetHealthPotionCount))
      (:%20%20
        (CallFunction|SetPotionCount _result)
        (CallFunction|SetHealth (+ 2e+01 (Variables|Default|GetcurrentHealth)))))))

(event Input|EnhancedActionEvents|EnhancedInputActionIA_Dash
  (params (ActionValue :type Boolean) (ElapsedSeconds :type Float%20%28double-precision%29) (TriggeredSeconds :type Float%20%28double-precision%29) (InputAction :type Input%20Action%20Object%20Reference :default "/Game/Input/Actions/IA_Dash.IA_Dash"))
  (:Started
    (bind _value (CallFunction|CheckCanDoAction 25.0))
    (if _value
      (Timeline|Dash PlayFromStart
        (:Update
          (Variables|/Script/Engine.MovementComponent|SetVelocity (Variables|Character|GetCharacterMovement) (* (Transformation|GetActorForwardVector) (Variables|Default|GetDashDistance))))
        (:Finished
          (CallFunction|SetStamina (- (Variables|Default|GetcurrentStamina) 25.0)))))))

(event Input|EnhancedActionEvents|EnhancedInputActionIA_GoToMainMenu
  (params (ActionValue :type Boolean) (ElapsedSeconds :type Float%20%28double-precision%29) (TriggeredSeconds :type Float%20%28double-precision%29) (InputAction :type Input%20Action%20Object%20Reference :default "/Game/Input/Actions/IA_GoToMainMenu.IA_GoToMainMenu"))
  (:Started
    (Input|SetInputModeUIOnly (Game|GetPlayerController 0) 0 "DoNotLock" false)
    (Game|OpenLevel(byObjectReference) "/Game/Maps/MainMenu.MainMenu")))

(event EventBeginPlay
  (CallFunction|InitPlayer))

(event EventTakeHealthPotion
  ;[1 1 1] Взаимодействие с зельями здоровья
  (bind _result (Math|Integer|IncrementInt (Variables|Default|GetHealthPotionCount))
    (:%20%20
      (CallFunction|SetPotionCount _result))))

(event EventTick
  (params (DeltaSeconds :type Float%20%28single-precision%29))
  (CallFunction|ChangeSprite)
  (if (< (Variables|Default|GetcurrentStamina) (Variables|Default|GetmaxStamina))
    (CallFunction|SetStamina (+ (Variables|Default|GetcurrentStamina) 0.25)))
  ;[1 1 1] Атака
  (if (Variables|Default|GetisAttacking)
    (if (== (Class|PaperFlipbookComponent|GetPlaybackPositioninFrames (Variables|Default|GetSprite)) 2)
      (Utilities|FlowControl|DoOnce false
        (:Completed
          (CallFunction|HitEnemies))))))

(event Game|Damage|EventAnyDamage
  (params (Damage :type Float%20%28single-precision%29) (DamageType :type Damage%20Type%20Object%20Reference) (InstigatedBy :type Controller%20Object%20Reference) (DamageCauser :type Actor%20Object%20Reference))
  (if (> (Variables|Default|GetcurrentHealth) 0.0)
    (CallFunction|SetDamage Damage)
    (if (<= (Variables|Default|GetcurrentHealth) 0.0)
      (CallFunction|Death))))

(event EventOnJumped
  ;[1 1 1] Прыжок / рестарт
  (CallFunction|SetStamina (- (Variables|Default|GetcurrentStamina) 2e+01)))

(event Collision|EventActorBeginOverlap
  (params (OtherActor :type Actor%20Object%20Reference))
  (if (Utilities|ClassIsChildOf (Utilities|GetClass OtherActor) "/Game/Blueprints/Items/Sword/BP_Sword.BP_Sword_C")
    (if (Utilities|DoesObjectImplementInterface OtherActor "/Game/Blueprints/BPI_Interact.BPI_Interact_C")
      (bind _texture (Class|BPIInteract|TakeLevelItem(Message) OtherActor))
      (Default|SetLevelItem (Variables|Default|GetWidgetUI) _texture)
      (Actor|DestroyActor OtherActor)
      (Variables|Default|SethasLevelItem true))))

(fn ConstructionScript)

(fn ChangeSprite
  (if (Variables|Default|GetisDead)
    (CallFunction|ChangeFlipbook false "/Game/Assets/Character/Death/Flipbook_Death.Flipbook_Death")
    (elif (Variables|Default|GetisAttacking)
      (CallFunction|ChangeFlipbook false "/Game/Assets/Character/Attack/Flipbook_Attack.Flipbook_Attack")
      (elif (AI|Components|NavMovement|IsMovingonGround (Variables|Character|GetCharacterMovement))
        (if (!= (.x (Transformation|GetVelocity)) 0.0)
          (CallFunction|ChangeFlipbook true "/Game/Assets/Character/Run/Flipbook_Run.Flipbook_Run")
          (else
            (CallFunction|ChangeFlipbook true "/Game/Assets/Character/Idle/Flipbook_Idle.Flipbook_Idle")))
        (else
          (CallFunction|ChangeFlipbook false "/Game/Assets/Character/Jump/Flipbook_Jump.Flipbook_Jump"))))))

(fn ChangeFlipbook
  (params (isLooping :type Boolean) (FlipBook :type Paper%20Flipbook%20Object%20Reference))
  (Components|Timeline|SetLooping (Variables|Default|GetSprite) isLooping)
  (Audio|Components|Audio|Play (Variables|Default|GetSprite))
  (Sprite|SetFlipbook (Variables|Default|GetSprite) FlipBook))

(fn InitPlayer
  (bind _maxstamina (Variables|Default|GetmaxStamina))
  (bind _maxhealth (Variables|Default|GetmaxHealth))
  (bind _asplayer_controller (Utilities|Casting|CastToPlayerController (Pawn|GetController)))
  (Input|AddMappingContext (PlayerController|LocalPlayerSubsystems|GetEnhancedInputLocalPlayerSubsystem _asplayer_controller) "/Game/Input/IMC_CharMove.IMC_CharMove" 0 "(bIgnoreAllPressedKeysUntilRelease=True,bForceImmediately=False,bNotifyUserSettings=False)")
  (Variables|Default|SetisAttacking false)
  (bind _output_get (Variables|Default|SetcurrentHealth _maxhealth))
  (bind _output_get_2 (Variables|Default|SetcurrentStamina _maxstamina))
  (bind _returnvalue (Game|GetCurrentLevelName true))
  (if (not (Utilities|Enum|Equal(Enum) _returnvalue "MainMenu"))
    ;[1 1 1] Создание UI для персонажа игрока
    (bind _returnvalue_2 (UserInterface|CreateWidget "/Game/UI/WB_Main.WB_Main_C" (Game|GetPlayerController 0)))
    (bind _output_get_3 (Variables|Default|SetWidgetUI _returnvalue_2))
    (UserInterface|Viewport|AddtoViewport _output_get_3 0)
    (Default|UpdateHealthUI (Variables|Default|GetWidgetUI) _output_get _maxhealth)
    (Default|UpdateStaminaUI (Variables|Default|GetWidgetUI) _output_get_2 _maxstamina)
    (CallFunction|SetPotionCount)))

(fn SetDamage
  (params (Damage :type Float%20%28double-precision%29))
  (CallFunction|SetHealth (- (Variables|Default|GetcurrentHealth) Damage)))

(fn HitEnemies
  (for _array_element (Collision|GetOverlappingActors (Variables|Default|GetHitbox) 0 :!class /Script/Engine.PrimitiveComponent)
    (if (!= _array_element self)
      (Game|Damage|ApplyDamage _array_element (Variables|Default|Getdamage) 0 0))))

(fn TakeHealthPotion
  (params (PotionCount :type Integer))
  (return 0))

(fn SetPotionCount
  (params (Count :type Integer))
  (bind _returnvalue (Math|Conversions|ToFloat(Integer) Count))
  (bind _returnvalue_2 (Math|Float|Clamp(Float) _returnvalue 0.0 1e+03))
  (bind _returnvalue_3 (Math|Float|Truncate _returnvalue_2))
  (Variables|Default|SetHealthPotionCount _returnvalue_3)
  (Default|UpdateHealthPotionCount (Variables|Default|GetWidgetUI) _returnvalue_3))

(fn SetHealth
  (params (Value :type Float%20%28double-precision%29))
  (bind _output_get (Variables|Default|SetcurrentHealth (Math|Float|Clamp(Float) Value 0.0 (Variables|Default|GetmaxHealth))))
  ;[1 1 1] Установка значения на полоске здоровья
  (Default|UpdateHealthUI (Variables|Default|GetWidgetUI) _output_get (Variables|Default|GetmaxHealth))
  (return (Variables|Default|GetcurrentHealth)))

(fn SetStamina
  (params (value :type Float%20%28double-precision%29))
  (bind _maxstamina (Variables|Default|GetmaxStamina))
  (bind _output_get (Variables|Default|SetcurrentStamina (Math|Float|Clamp(Float) value 0.0 _maxstamina)))
  (Default|UpdateStaminaUI (Variables|Default|GetWidgetUI) _output_get _maxstamina)
  (return (Variables|Default|GetcurrentStamina)))

(fn CheckCanDoAction
  (params (NeededStamina :type Float%20%28double-precision%29))
  (if (or (Variables|Default|GetisAttacking) (Variables|Default|GetisDead))
    (return false)
    (elif (> (Variables|Default|GetcurrentStamina) NeededStamina)
      (return true)
      (else
        (return false)))))

(fn RestartLevel
  (bind _returnvalue (Game|GetCurrentLevelName true))
  (Game|OpenLevel(byName) (Utilities|String|StringToName _returnvalue)))

(fn CheckHasLevelItem
  (return (Variables|Default|GethasLevelItem)))

(fn TakeLevelItem
  (return ""))