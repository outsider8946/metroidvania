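; BP_Teleport is an overlap-triggered level exit that sends the player to the MainMenu level if they hold the required level item.
; When the player pawn overlaps it, a WB_Dialog widget appears and the BPI_hasLevelItem interface queries the pawn for the item.
; The result selects a DialogText line; after a short delay, it either opens the level or removes the dialog.
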(event EventBeginPlay)

(event EventTick
  (params (DeltaSeconds :type Float%20%28single-precision%29)))

(event Collision|EventActorBeginOverlap
  (params (OtherActor :type Actor%20Object%20Reference))
  (bind _returnvalue (Game|Player|GetPlayerPawn 0))
  (if (== OtherActor (Game|Player|GetPlayerPawn 0))
    (bind _returnvalue_2 (UserInterface|CreateWidget "/Game/UI/WB_Dialog.WB_Dialog_C" (Game|GetPlayerController 0)))
    (UserInterface|Viewport|AddtoViewport _returnvalue_2 0)
    (if (Utilities|DoesObjectImplementInterface _returnvalue "/Game/Blueprints/Items/TeleportToSecondLevel/BPI_hasLevelItem.BPI_hasLevelItem_C")
      (bind _value (Class|BPIHasLevelItem|CheckHasLevelItem(Message) _returnvalue))
      (if _value
        (Default|ShowDialogText _returnvalue_2 (Utilities|Array|Get(acopy) (Variables|Default|GetDialogText) 1))
        (Utilities|FlowControl|Delay 3.0)
        (Game|OpenLevel(byObjectReference) "/Game/Maps/MainMenu.MainMenu")
        (else
          (Default|ShowDialogText _returnvalue_2 (Utilities|Array|Get(acopy) (Variables|Default|GetDialogText)))
          (Utilities|FlowControl|Delay 3.0)
          (Widget|RemovefromParent _returnvalue_2))))))

(fn ConstructionScript)