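; BP_Skeleton is a 2D Paper2D skeleton enemy with health, damage handling and flipbook-driven animation.
; Incoming damage lowers clamped health, and reaching zero sets IsDead and writes it to the AI controller's blackboard.
; Every tick, ChangeSprite picks the death, hit, move or idle flipbook from the dead and attacking flags and horizontal velocity, looping only move and idle.
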(event Custom|Death
  (bind _output_get (Variables|Default|SetisDead true))
  (AI|Components|Blackboard|SetValueasBool (AI|GetBlackboard (AI|GetAIController self)) (Utilities|Name|MakeLiteralName "isDead") _output_get))

(event EventBeginPlay
  (Variables|Default|SetcurrentHealth (Variables|Default|GetmaxHealth)))

(event Collision|EventActorBeginOverlap
  (params (OtherActor :type Actor%20Object%20Reference)))

(event EventTick
  (params (DeltaSeconds :type Float%20%28single-precision%29))
  (CallFunction|ChangeSprite))

(event Game|Damage|EventAnyDamage
  (params (Damage :type Float%20%28single-precision%29) (DamageType :type Damage%20Type%20Object%20Reference) (InstigatedBy :type Controller%20Object%20Reference) (DamageCauser :type Actor%20Object%20Reference))
  (CallFunction|SetDamage Damage)
  (if (<= (Variables|Default|GetcurrentHealth) 0.0)
    (CallFunction|Death)))

(fn ConstructionScript)

(fn ChangeFlipbook
  (params (isLooping :type Boolean) (FlipBook :type Paper%20Flipbook%20Object%20Reference))
  (Components|Timeline|SetLooping (Variables|Default|GetSprite) isLooping)
  (Audio|Components|Audio|Play (Variables|Default|GetSprite))
  (Sprite|SetFlipbook (Variables|Default|GetSprite) FlipBook))

(fn ChangeSprite
  (if (Variables|Default|GetisDead)
    (CallFunction|ChangeFlipbook false "/Game/Assets/Enemies/Skeleton/Death/Flipbook_Death.Flipbook_Death")
    (elif (Variables|Default|GetisAttacking)
      (CallFunction|ChangeFlipbook false "/Game/Assets/Enemies/Skeleton/Attack/Flipbook_Hit.Flipbook_Hit")
      (elif (!= (.x (Transformation|GetVelocity)) 0.0)
        (CallFunction|ChangeFlipbook true "/Game/Assets/Enemies/Skeleton/Move/Flipbook_Move.Flipbook_Move")
        (else
          (CallFunction|ChangeFlipbook true "/Game/Assets/Enemies/Skeleton/Idle/Flipbook_Idle.Flipbook_Idle"))))))

(fn SetDamage
  (params (Damage :type Float%20%28double-precision%29))
  (Variables|Default|SetcurrentHealth (Math|Float|Clamp(Float) (- (Variables|Default|GetcurrentHealth) Damage) 0.0 (Variables|Default|GetmaxHealth))))