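; BP_Skeleton is a 2D skeleton enemy that chases the player, attacks, defends and dies.
; Pawn sensing and death set AI blackboard keys, alongside range values written at start.
; Tick picks the Paper2D flipbook from dead, defending, attacking and velocity states.
; Attack, when called on flipbook frame 6, damages overlapping non-self actors once until playback finishes; defending ignores incoming damage.
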(event OnFinishedPlaying(Sprite)
  ;[1 1 1] Ресет состояний после окончания проигрывания анимаций
  (if (== (Variables|Default|GetisAttacking) true)
    (Variables|Default|SetisAttacking false)
    (CallFunction|ResetAttack)))

(event OnSeePawn(PawnSensing)
  (params (Pawn :type Pawn%20Object%20Reference))
  ;[1 1 1] Преследование
  (if (== Pawn (Game|Player|GetPlayerPawn 0))
    (bind _output_get (Variables|Default|SetisChasingPlayer true))
    (AI|Components|Blackboard|SetValueasBool (Variables|/Script/AIModule.AIController|GetBlackboard (AI|GetAIController self)) (Utilities|Name|MakeLiteralName "isChasingPlayer") _output_get)))

(event Custom|Death
  (bind _output_get (Variables|Default|SetisDead true))
  (AI|Components|Blackboard|SetValueasBool (AI|GetBlackboard (AI|GetAIController self)) (Utilities|Name|MakeLiteralName "isDead") _output_get))

(event Custom|Reset%20Attack
  ;[1 1 1] Атака
  (Utilities|FlowControl|DoOnce false) ; enters at Reset
)

(event EventBeginPlay
  (CallFunction|Init))

(event Collision|EventActorBeginOverlap
  (params (OtherActor :type Actor%20Object%20Reference)))

(event EventTick
  (params (DeltaSeconds :type Float%20%28single-precision%29))
  (CallFunction|ChangeSprite))

(event Game|Damage|EventAnyDamage
  (params (Damage :type Float%20%28single-precision%29) (DamageType :type Damage%20Type%20Object%20Reference) (InstigatedBy :type Controller%20Object%20Reference) (DamageCauser :type Actor%20Object%20Reference))
  (if (not (Variables|Default|GetisDefending))
    (CallFunction|SetDamage Damage)
    (if (<= (Variables|Default|GetcurrentHealth) 0.0)
      (CallFunction|Death))))

(event EventAttack
  ;[1 1 1] Атака
  (Variables|Default|SetisDefending false)
  (Variables|Default|SetisAttacking true)
  (if (== (Class|PaperFlipbookComponent|GetPlaybackPositioninFrames (Variables|Default|GetSprite)) 6)
    (Utilities|FlowControl|DoOnce false
      (:Completed
        (CallFunction|HitEnemies)))))

(event EventDefend
  (params (Value :type Boolean))
  ;[1 1 1] Защита
  (Variables|Default|SetisAttacking false)
  (Variables|Default|SetisDefending Value))

(fn ConstructionScript)

(fn ChangeFlipbook
  (params (isLooping :type Boolean) (FlipBook :type Paper%20Flipbook%20Object%20Reference))
  (Components|Timeline|SetLooping (Variables|Default|GetSprite) isLooping)
  (Audio|Components|Audio|Play (Variables|Default|GetSprite))
  (Sprite|SetFlipbook (Variables|Default|GetSprite) FlipBook))

(fn ChangeSprite
  (if (Variables|Default|GetisDead)
    (CallFunction|ChangeFlipbook false "/Game/Assets/Enemies/Skeleton/Death/Flipbook_Death.Flipbook_Death")
    (elif (Variables|Default|GetisDefending)
      (CallFunction|ChangeFlipbook true "/Game/Assets/Enemies/Skeleton/Defend/Flipbook_Defend.Flipbook_Defend")
      (elif (Variables|Default|GetisAttacking)
        (CallFunction|ChangeFlipbook false "/Game/Assets/Enemies/Skeleton/Attack/Flipbook_Attack.Flipbook_Attack")
        (elif (!= (.x (Transformation|GetVelocity)) 0.0)
          (CallFunction|ChangeFlipbook true "/Game/Assets/Enemies/Skeleton/Move/Flipbook_Move.Flipbook_Move")
          (else
            (CallFunction|ChangeFlipbook true "/Game/Assets/Enemies/Skeleton/Idle/Flipbook_Idle.Flipbook_Idle")))))))

(fn SetDamage
  (params (Damage :type Float%20%28double-precision%29))
  (Variables|Default|SetcurrentHealth (Math|Float|Clamp(Float) (- (Variables|Default|GetcurrentHealth) Damage) 0.0 (Variables|Default|GetmaxHealth))))

(fn HitEnemies
  (for _array_element (Collision|GetOverlappingActors (Variables|Default|GetHitbox) 0 :!class /Script/Engine.PrimitiveComponent)
    (if (or (!= _array_element self) (== _array_element (Game|Player|GetPlayerPawn 0)))
      (Game|Damage|ApplyDamage _array_element (Variables|Default|Getdamage) 0 0))))

(fn Init
  (bind _self self)
  (bind _returnvalue (AI|GetAIController _self))
  (bind _blackboard (Variables|/Script/AIModule.AIController|GetBlackboard _returnvalue))
  (Variables|Default|SetcurrentHealth (Variables|Default|GetmaxHealth))
  (Variables|Default|SetattackModeRange 1e+02)
  (bind _output_get (Variables|Default|SethitboxRange 7e+01))
  (AI|Components|Blackboard|SetValueasFloat _blackboard (Utilities|Name|MakeLiteralName "hitboxRange") _output_get)
  (AI|Components|Blackboard|SetValueasFloat _blackboard (Utilities|Name|MakeLiteralName "attackModeRange") (Variables|Default|GetattackModeRange)))